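; Shaped color-correction volume actor that grades the image through a post-process blendable material.
; The construction script runs UpdateVolume, which, when enabled and visible, picks a parent material for sphere, box, cylinder or cone.
; It switches to advanced material variants only when shadow, midtone or highlight grading differs from neutral, though cylinder always uses one material.
; A dynamic instance receives the transform, falloff and grading parameters.
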(event EventBeginPlay)

(event Collision|EventActorBeginOverlap
  (params (OtherActor :type Actor%20Object%20Reference)))

(event EventTick
  (params (DeltaSeconds :type Float%20%28single-precision%29)))

(fn ConstructionScript
  (CallFunction|UpdateVolume))

(fn CheckAdvancedColorCorrectDefaults
  (bind _linearcolor (Utilities|Struct|MakeLinearColor 1.0 1.0 1.0 1.0))
  (bind _linearcolor_2 (Utilities|Struct|MakeLinearColor 0.0 0.0 0.0 0.0))
  (bind _colorcorrect (Variables|Default|GetColorCorrect))
  (bind (_global _shadows _midtones _highlights) (Utilities|Struct|BreakColorGradingSettings _colorcorrect))
  (bind (_saturation _contrast _gamma _gain _offset) (Utilities|Struct|BreakColorGradePerRangeSettings _shadows))
  (bind (_saturation_2 _contrast_2 _gamma_2 _gain_2 _offset_2) (Utilities|Struct|BreakColorGradePerRangeSettings _highlights))
  (bind (_saturation_3 _contrast_3 _gamma_3 _gain_3 _offset_3) (Utilities|Struct|BreakColorGradePerRangeSettings _midtones))
  (Variables|Default|SetEnableAdvancedCC (not (Math|Boolean|ANDBoolean (Math|Boolean|ANDBoolean (== _linearcolor (Utilities|Struct|MakeLinearColor (.x _saturation) (.y _saturation) (.z _saturation) (.w _saturation))) (== _linearcolor (Utilities|Struct|MakeLinearColor (.x _contrast) (.y _contrast) (.z _contrast) (.w _contrast))) (== _linearcolor (Utilities|Struct|MakeLinearColor (.x _gamma) (.y _gamma) (.z _gamma) (.w _gamma))) (== _linearcolor (Utilities|Struct|MakeLinearColor (.x _gain) (.y _gain) (.z _gain) (.w _gain))) (== _linearcolor_2 (Utilities|Struct|MakeLinearColor (.x _offset) (.y _offset) (.z _offset) (.w _offset)))) (Math|Boolean|ANDBoolean (== _linearcolor (Utilities|Struct|MakeLinearColor (.x _saturation_3) (.y _saturation_3) (.z _saturation_3) (.w _saturation_3))) (== _linearcolor (Utilities|Struct|MakeLinearColor (.x _contrast_3) (.y _contrast_3) (.z _contrast_3) (.w _contrast_3))) (== _linearcolor (Utilities|Struct|MakeLinearColor (.x _gamma_3) (.y _gamma_3) (.z _gamma_3) (.w _gamma_3))) (== _linearcolor (Utilities|Struct|MakeLinearColor (.x _gain_3) (.y _gain_3) (.z _gain_3) (.w _gain_3))) (== _linearcolor_2 (Utilities|Struct|MakeLinearColor (.x _offset_3) (.y _offset_3) (.z _offset_3) (.w _offset_3)))) (Math|Boolean|ANDBoolean (== _linearcolor (Utilities|Struct|MakeLinearColor (.x _saturation_2) (.y _saturation_2) (.z _saturation_2) (.w _saturation_2))) (== _linearcolor (Utilities|Struct|MakeLinearColor (.x _contrast_2) (.y _contrast_2) (.z _contrast_2) (.w _contrast_2))) (== _linearcolor (Utilities|Struct|MakeLinearColor (.x _gamma_2) (.y _gamma_2) (.z _gamma_2) (.w _gamma_2))) (== _linearcolor (Utilities|Struct|MakeLinearColor (.x _gain_2) (.y _gain_2) (.z _gain_2) (.w _gain_2))) (== _linearcolor_2 (Utilities|Struct|MakeLinearColor (.x _offset_2) (.y _offset_2) (.z _offset_2) (.w _offset_2))))))))

(fn UpdateVolume
  (bind _enableadvancedcc (Variables|Default|GetEnableAdvancedCC))
  (bind _inner (Variables|Default|GetInner))
  (bind _outer (Variables|Default|GetOuter))
  (bind _colorcorrect (Variables|Default|GetColorCorrect))
  (bind _defaultsceneroot (Variables|Default|GetDefaultSceneRoot))
  (bind (_global _shadows _midtones _highlights _shadowsmax _highlightsmin) (Utilities|Struct|BreakColorGradingSettings _colorcorrect))
  (bind _returnvalue (Transformation|GetWorldRotation _defaultsceneroot))
  (bind (_saturation _contrast _gamma _gain _offset) (Utilities|Struct|BreakColorGradePerRangeSettings _global))
  (bind (_saturation_2 _contrast_2 _gamma_2 _gain_2 _offset_2) (Utilities|Struct|BreakColorGradePerRangeSettings _shadows))
  (bind (_saturation_3 _contrast_3 _gamma_3 _gain_3 _offset_3) (Utilities|Struct|BreakColorGradePerRangeSettings _highlights))
  (bind (_saturation_4 _contrast_4 _gamma_4 _gain_4 _offset_4) (Utilities|Struct|BreakColorGradePerRangeSettings _midtones))
  (if (and (Variables|Default|GetEnabled) (not (Variables|Rendering|GetbHidden)))
    (CallFunction|CheckAdvancedColorCorrectDefaults)
    (switch Utilities|FlowControl|Switch|SwitchonEnum_SimpleCCVType (Variables|Default|GetType)
      (:NewEnumerator0
        (Rendering|SetVisibility (Variables|Default|GetSphere) true false)
        (if _enableadvancedcc
          (Variables|Default|SetMaterialInstanceParent "/SimpleVirtualProduction/CCV/M_ColorCorrectVolume_AdvCC.M_ColorCorrectVolume_AdvCC")
          (else
            (Variables|Default|SetMaterialInstanceParent "/SimpleVirtualProduction/CCV/M_ColorCorrectVolume.M_ColorCorrectVolume"))))
      (:NewEnumerator1
        (Rendering|SetVisibility (Variables|Default|GetBox) true false)
        (if _enableadvancedcc
          (Variables|Default|SetMaterialInstanceParent "/SimpleVirtualProduction/CCV/M_ColorCorrectVolume_Box_AdvCC.M_ColorCorrectVolume_Box_AdvCC")
          (else
            (Variables|Default|SetMaterialInstanceParent "/SimpleVirtualProduction/CCV/M_ColorCorrectVolume_Box.M_ColorCorrectVolume_Box"))))
      (:NewEnumerator2
        (Rendering|SetVisibility (Variables|Default|GetCylinder) true false)
        (if _enableadvancedcc
          (Variables|Default|SetMaterialInstanceParent "/SimpleVirtualProduction/CCV/M_ColorCorrectVolume_Cylinder.M_ColorCorrectVolume_Cylinder")
          (else
            (Variables|Default|SetMaterialInstanceParent "/SimpleVirtualProduction/CCV/M_ColorCorrectVolume_Cylinder.M_ColorCorrectVolume_Cylinder"))))
      (:NewEnumerator3
        (Rendering|SetVisibility (Variables|Default|GetCone) true false)
        (if _enableadvancedcc
          (Variables|Default|SetMaterialInstanceParent "/SimpleVirtualProduction/CCV/M_ColorCorrectVolume_Cone_AdvCC.M_ColorCorrectVolume_Cone_AdvCC")
          (else
            (Variables|Default|SetMaterialInstanceParent "/SimpleVirtualProduction/CCV/M_ColorCorrectVolume_Cone.M_ColorCorrectVolume_Cone")))))
    (bind _returnvalue_2 (Rendering|Material|CreateDynamicMaterialInstance (Variables|Default|GetMaterialInstanceParent) "None" "None" :!class /Script/Engine.KismetMaterialLibrary))
    (bind _output_get (Variables|Default|SetMID _returnvalue_2))
    (Variables|/Script/Engine.PostProcessComponent|SetSettings (Variables|Default|GetPostProcess) (Utilities|Struct|MakePostProcessSettings (Utilities|Struct|MakeWeightedBlendables (Utilities|Array|MakeArray (Utilities|Struct|MakeWeightedBlendable 1.0 _output_get)))))
    (Rendering|Material|SetVectorParameterValue (Variables|Default|GetMID) "Translate" (Math|Conversions|ToLinearColor(Vector) (Transformation|GetWorldLocation (Variables|Default|GetDefaultSceneRoot))) :!class /Script/Engine.MaterialInstanceDynamic)
    (Rendering|Material|SetVectorParameterValue (Variables|Default|GetMID) "Rotate" (Math|Conversions|ToLinearColor(Vector) (Math|Vector|MakeVector (.roll _returnvalue) (.pitch _returnvalue) (.yaw _returnvalue))) :!class /Script/Engine.MaterialInstanceDynamic)
    (Rendering|Material|SetVectorParameterValue (Variables|Default|GetMID) "Scale" (Math|Conversions|ToLinearColor(Vector) (Transformation|GetWorldScale (Variables|Default|GetDefaultSceneRoot))) :!class /Script/Engine.MaterialInstanceDynamic)
    (Rendering|Material|SetScalarParameterValue (Variables|Default|GetMID) "Intensity" (Variables|Default|GetIntensity) :!class /Script/Engine.MaterialInstanceDynamic)
    (if (< _inner _outer)
      (Rendering|Material|SetScalarParameterValue (Variables|Default|GetMID) "Inner" _inner :!class /Script/Engine.MaterialInstanceDynamic)
      (Rendering|Material|SetScalarParameterValue (Variables|Default|GetMID) "Outer" _outer :!class /Script/Engine.MaterialInstanceDynamic)
      (else
        (Rendering|Material|SetScalarParameterValue (Variables|Default|GetMID) "Inner" _outer :!class /Script/Engine.MaterialInstanceDynamic)
        (Rendering|Material|SetScalarParameterValue (Variables|Default|GetMID) "Outer" _inner :!class /Script/Engine.MaterialInstanceDynamic)))
    (Rendering|Material|SetScalarParameterValue (Variables|Default|GetMID) "Falloff" (Variables|Default|GetFalloff) :!class /Script/Engine.MaterialInstanceDynamic)
    (Rendering|Material|SetScalarParameterValue (Variables|Default|GetMID) "Invert" (Math|Conversions|ToFloat(Boolean) (Variables|Default|GetInvert)) :!class /Script/Engine.MaterialInstanceDynamic)
    (Rendering|Material|SetScalarParameterValue (Variables|Default|GetMID) "FakeLight" (Variables|Default|GetFakeLight) :!class /Script/Engine.MaterialInstanceDynamic)
    (Rendering|Material|SetScalarParameterValue (Variables|Default|GetMID) "WhiteTemp" (Variables|Default|GetTemp) :!class /Script/Engine.MaterialInstanceDynamic)
    (Rendering|Material|SetVectorParameterValue (Variables|Default|GetMID) "ArrowDirection" (Math|Conversions|ToLinearColor(Vector) (Math|Vector|GetForwardVector (Variables|Default|GetArrow))) :!class /Script/Engine.MaterialInstanceDynamic)
    (Rendering|Material|SetScalarParameterValue (Variables|Default|GetMID) "ExcludeStencil" (Math|Conversions|ToFloat(Boolean) (Variables|Default|GetExcludeStencil)) :!class /Script/Engine.MaterialInstanceDynamic)
    (switch Utilities|FlowControl|Switch|SwitchonEnum_SimpleCCVType (Variables|Default|GetType)
      (:NewEnumerator0
        (Rendering|Material|SetScalarParameterValue (Variables|Default|GetMID) "Shape" 0.0 :!class /Script/Engine.MaterialInstanceDynamic))
      (:NewEnumerator1
        (Rendering|Material|SetScalarParameterValue (Variables|Default|GetMID) "Shape" 1.0 :!class /Script/Engine.MaterialInstanceDynamic))
      (:NewEnumerator2
        (Rendering|Material|SetScalarParameterValue (Variables|Default|GetMID) "Shape" 2.0 :!class /Script/Engine.MaterialInstanceDynamic))
      (:NewEnumerator3
        (Rendering|Material|SetScalarParameterValue (Variables|Default|GetMID) "Shape" 3.0 :!class /Script/Engine.MaterialInstanceDynamic)))
    (Rendering|Material|SetVectorParameterValue (Variables|Default|GetMID) "ColorSaturationMaster" (Utilities|Struct|MakeLinearColor (.x _saturation) (.y _saturation) (.z _saturation) (.w _saturation)) :!class /Script/Engine.MaterialInstanceDynamic)
    (Rendering|Material|SetVectorParameterValue (Variables|Default|GetMID) "ColorContrastMaster" (Utilities|Struct|MakeLinearColor (.x _contrast) (.y _contrast) (.z _contrast) (.w _contrast)) :!class /Script/Engine.MaterialInstanceDynamic)
    (Rendering|Material|SetVectorParameterValue (Variables|Default|GetMID) "ColorGammaMaster" (Utilities|Struct|MakeLinearColor (.x _gamma) (.y _gamma) (.z _gamma) (.w _gamma)) :!class /Script/Engine.MaterialInstanceDynamic)
    (Rendering|Material|SetVectorParameterValue (Variables|Default|GetMID) "ColorGainMaster" (Utilities|Struct|MakeLinearColor (.x _gain) (.y _gain) (.z _gain) (.w _gain)) :!class /Script/Engine.MaterialInstanceDynamic)
    (Rendering|Material|SetVectorParameterValue (Variables|Default|GetMID) "ColorOffsetMaster" (Utilities|Struct|MakeLinearColor (.x _offset) (.y _offset) (.z _offset) (.w _offset)) :!class /Script/Engine.MaterialInstanceDynamic)
    (if (Variables|Default|GetEnableAdvancedCC)
      (Rendering|Material|SetVectorParameterValue (Variables|Default|GetMID) "ColorSaturationShadows" (Utilities|Struct|MakeLinearColor (.x _saturation_2) (.y _saturation_2) (.z _saturation_2) (.w _saturation_2)) :!class /Script/Engine.MaterialInstanceDynamic)
      (Rendering|Material|SetVectorParameterValue (Variables|Default|GetMID) "ColorContrastShadows" (Utilities|Struct|MakeLinearColor (.x _contrast_2) (.y _contrast_2) (.z _contrast_2) (.w _contrast_2)) :!class /Script/Engine.MaterialInstanceDynamic)
      (Rendering|Material|SetVectorParameterValue (Variables|Default|GetMID) "ColorGammaShadows" (Utilities|Struct|MakeLinearColor (.x _gamma_2) (.y _gamma_2) (.z _gamma_2) (.w _gamma_2)) :!class /Script/Engine.MaterialInstanceDynamic)
      (Rendering|Material|SetVectorParameterValue (Variables|Default|GetMID) "ColorGainShadows" (Utilities|Struct|MakeLinearColor (.x _gain_2) (.y _gain_2) (.z _gain_2) (.w _gain_2)) :!class /Script/Engine.MaterialInstanceDynamic)
      (Rendering|Material|SetVectorParameterValue (Variables|Default|GetMID) "ColorOffsetShadows" (Utilities|Struct|MakeLinearColor (.x _offset_2) (.y _offset_2) (.z _offset_2) (.w _offset_2)) :!class /Script/Engine.MaterialInstanceDynamic)
      (Rendering|Material|SetVectorParameterValue (Variables|Default|GetMID) "ColorSaturationMidtones" (Utilities|Struct|MakeLinearColor (.x _saturation_4) (.y _saturation_4) (.z _saturation_4) (.w _saturation_4)) :!class /Script/Engine.MaterialInstanceDynamic)
      (Rendering|Material|SetVectorParameterValue (Variables|Default|GetMID) "ColorContrastMidtones" (Utilities|Struct|MakeLinearColor (.x _contrast_4) (.y _contrast_4) (.z _contrast_4) (.w _contrast_4)) :!class /Script/Engine.MaterialInstanceDynamic)
      (Rendering|Material|SetVectorParameterValue (Variables|Default|GetMID) "ColorGammaMidtones" (Utilities|Struct|MakeLinearColor (.x _gamma_4) (.y _gamma_4) (.z _gamma_4) (.w _gamma_4)) :!class /Script/Engine.MaterialInstanceDynamic)
      (Rendering|Material|SetVectorParameterValue (Variables|Default|GetMID) "ColorGainMidtones" (Utilities|Struct|MakeLinearColor (.x _gain_4) (.y _gain_4) (.z _gain_4) (.w _gain_4)) :!class /Script/Engine.MaterialInstanceDynamic)
      (Rendering|Material|SetVectorParameterValue (Variables|Default|GetMID) "ColorOffsetMidtones" (Utilities|Struct|MakeLinearColor (.x _offset_4) (.y _offset_4) (.z _offset_4) (.w _offset_4)) :!class /Script/Engine.MaterialInstanceDynamic)
      (Rendering|Material|SetVectorParameterValue (Variables|Default|GetMID) "ColorSaturationHighlights" (Utilities|Struct|MakeLinearColor (.x _saturation_3) (.y _saturation_3) (.z _saturation_3) (.w _saturation_3)) :!class /Script/Engine.MaterialInstanceDynamic)
      (Rendering|Material|SetVectorParameterValue (Variables|Default|GetMID) "ColorContrastHighlights" (Utilities|Struct|MakeLinearColor (.x _contrast_3) (.y _contrast_3) (.z _contrast_3) (.w _contrast_3)) :!class /Script/Engine.MaterialInstanceDynamic)
      (Rendering|Material|SetVectorParameterValue (Variables|Default|GetMID) "ColorGammaHightlights" (Utilities|Struct|MakeLinearColor (.x _gamma_3) (.y _gamma_3) (.z _gamma_3) (.w _gamma_3)) :!class /Script/Engine.MaterialInstanceDynamic)
      (Rendering|Material|SetVectorParameterValue (Variables|Default|GetMID) "ColorGainHightlights" (Utilities|Struct|MakeLinearColor (.x _gain_3) (.y _gain_3) (.z _gain_3) (.w _gain_3)) :!class /Script/Engine.MaterialInstanceDynamic)
      (Rendering|Material|SetVectorParameterValue (Variables|Default|GetMID) "ColorOffsetHighlights" (Utilities|Struct|MakeLinearColor (.x _offset_3) (.y _offset_3) (.z _offset_3) (.w _offset_3)) :!class /Script/Engine.MaterialInstanceDynamic)
      (Rendering|Material|SetScalarParameterValue (Variables|Default|GetMID) "ShadowMax" _shadowsmax :!class /Script/Engine.MaterialInstanceDynamic)
      (Rendering|Material|SetScalarParameterValue (Variables|Default|GetMID) "HighlightMin" _highlightsmin :!class /Script/Engine.MaterialInstanceDynamic))))