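; Blueprint function library of small helpers for virtual production.
; DetermineForegroundColor picks white or black Slate text by the background's RGB distance from white, biased toward black.
; OffsetTransform moves a transform along its own forward and up vectors.
; UpdateScreenSizeFromFilmback rescales a screen mesh and component from the cine camera's filmback aspect, using 16:9 as the component baseline and multiplying current scales, so repeated calls compound.
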(fn DetermineForegroundColor
  (params (BackgroundColor :type Linear%20Color%20Structure) (__WorldContext :type Object%20Object%20Reference))
  (bind (_r _g _b) (Utilities|Struct|BreakLinearColor BackgroundColor))
  (return (select (>= (Math|Vector|VectorLength (- "1.000000,1.000000,1.000000" (Math|Vector|MakeVector _r _g _b))) 1.2) (Utilities|Struct|MakeSlateColor "(R=1.000000,G=1.000000,B=1.000000,A=1.000000)") (Utilities|Struct|MakeSlateColor "(R=0.000000,G=0.000000,B=0.000000,A=1.000000)"))))

(fn OffsetTransform
  (params (StartTransform :type Transform) (ForwardOffset :type Float%20%28single-precision%29) (UpOffset :type Float%20%28single-precision%29) (__WorldContext :type Object%20Object%20Reference))
  (bind (_location _rotation _scale) (Math|Transform|BreakTransform StartTransform))
  (return (Math|Transform|MakeTransform (+ (* (Math|Vector|Normalize (Math|Vector|GetForwardVector _rotation)) ForwardOffset) _location (* (Math|Vector|Normalize (Math|Vector|GetUpVector _rotation)) UpOffset)) _rotation _scale)))

(fn UpdateScreenSizefromFilmback
  (params (ScreenMeshToScale :type Static%20Mesh%20Component%20Object%20Reference) (ScreenComponent :type Scene%20Component%20Object%20Reference) (CineCameraComponent :type Cine%20Camera%20Component%20Object%20Reference) (__WorldContext :type Object%20Object%20Reference))
  (bind _filmback (Variables|/Script/CinematicCamera.CineCameraComponent|GetFilmback CineCameraComponent))
  (bind _relativescale3d (Variables|/Script/Engine.SceneComponent|GetRelativeScale3D ScreenMeshToScale))
  (bind (_sensorwidth _sensorheight) (Utilities|Struct|BreakCameraFilmbackSettings _filmback))
  (bind (_x _y _z) (Math|Vector|BreakVector _relativescale3d))
  (bind _returnvalue (/ _sensorwidth _sensorheight))
  (Transformation|SetRelativeScale3D ScreenMeshToScale (Math|Vector|MakeVector _x _y (/ _z _returnvalue)))
  (Transformation|SetRelativeScale3D ScreenComponent (* (Variables|/Script/Engine.SceneComponent|GetRelativeScale3D ScreenComponent) (/ _returnvalue 1.777778))))