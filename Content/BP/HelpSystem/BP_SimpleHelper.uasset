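; VR editor help callout that shows a text label at the end of a leader line, opened for a VR tool.
; Construction and first tick size the spline-mesh line, text and background from text length, scale and alignment.
; EditorTick turns the label toward the headset and eases actor scale up to world scale when within distance and view-direction thresholds, otherwise to zero.
; Closing shrinks the actor, then destroys it.
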(event Custom|Refresh
  (CallFunction|UpdateHelperParameters)
  (Transformation|SetActorScale3D "0, 0, 0"))

(event Custom|Close
  (Variables|Logic|SetEnabled false))

(event Custom|Open
  (params (VRTool :type Simple%20VR%20Tool%20BP%20Object%20Reference))
  (Variables|Logic|SetEnabled true)
  (Variables|Default|SetVRTool VRTool))

(event Custom|Flip%20Text
  (Transformation|SetRelativeScale3D (Variables|Default|GetTextRender) "1.000000,-1.000000,1.000000"))

(event EventEditorTick
  (params (DeltaSeconds :type Float%20%28single-precision%29))
  (bind _returnvalue (Transformation|GetActorTransform))
  (bind _returnvalue_2 (Transformation|GetActorScale3D))
  (bind _vrtool (Variables|Default|GetVRTool))
  (bind _base (Variables|Default|GetBase))
  (bind _returnvalue_3 (SplineMesh|GetEndPosition _base))
  (bind _returnvalue_4 (Math|Interpolation|VInterpTo _returnvalue_2 "0, 0, 0" DeltaSeconds 1e+01))
  (bind _parentinteractor (Variables|/SimpleVirtualProduction/VRTools/SimpleVRTool_BP.SimpleVRTool_BP_C|GetParentInteractor _vrtool))
  (bind _returnvalue_5 (Math|Transform|TransformLocation _returnvalue _returnvalue_3))
  (bind _returnvalue_6 (Class|ViewportInteractor|GetWorldInteraction _parentinteractor))
  (bind _returnvalue_7 (Class|ViewportWorldInteraction|GetWorldScaleFactor _returnvalue_6))
  (bind _returnvalue_8 (Class|VPBlueprintLibrary|IsVREditorModeActive))
  (if _returnvalue_8
    (if (Variables|Logic|GetEnabled)
      (Utilities|FlowControl|Sequence
        (:then_0
          (Utilities|FlowControl|DoOnce false
            (:Completed
              (CallFunction|Refresh)
              (Collision|SetActorEnableCollision false))))
        (:then_1
          (Transformation|SetWorldLocation (Variables|Default|GetT_TextUnderline) _returnvalue_5 false false)
          (bind _returnvalue_9 (Class|SimpleVPBlueprintLibrary|GetEditorVRHeadTransform))
          (Transformation|SetWorldRotation (Variables|Default|GetT_TextUnderline) (Math|Rotator|MakeRotator 0.0 (.pitch (Math|Rotator|FindLookatRotation _returnvalue_5 (.location _returnvalue_9))) (.yaw (Math|Rotator|FindLookatRotation _returnvalue_5 (.location _returnvalue_9)))) false false)
          (bind _returnvalue_10 (Class|SimpleVPBlueprintLibrary|GetEditorVRHeadTransform))
          (Utilities|IsValid (Variables|Default|GetVRTool)
            (:Is%20Valid
              (Transformation|SetActorScale3D (Math|Interpolation|VInterpTo (Transformation|GetActorScale3D) (select (and (<= (Math|Vector|VectorLength (- (.location _returnvalue_10) (Transformation|GetActorLocation))) (* (Variables|Default|GetDistanceThreshold) _returnvalue_7)) (<= (Math|Vector|DotProduct (Math|Vector|GetForwardVector (.rotation _returnvalue_10)) (Math|Vector|GetForwardVector (Variables|Default|GetArrow))) (Variables|Logic|GetDotThreshold))) (Math|Conversions|ToVector(Float) _returnvalue_7) "0, 0, 0") DeltaSeconds 1e+01))
              (Rendering|SetVisibility (Variables|Default|GetSM_BG_Center) (not (and (Math|Vector|Equal(Vector) (Math|Interpolation|VInterpTo (Transformation|GetActorScale3D) (select (and (<= (Math|Vector|VectorLength (- (.location _returnvalue_10) (Transformation|GetActorLocation))) (* (Variables|Default|GetDistanceThreshold) _returnvalue_7)) (<= (Math|Vector|DotProduct (Math|Vector|GetForwardVector (.rotation _returnvalue_10)) (Math|Vector|GetForwardVector (Variables|Default|GetArrow))) (Variables|Logic|GetDotThreshold))) (Math|Conversions|ToVector(Float) _returnvalue_7) "0, 0, 0") DeltaSeconds 1e+01) "0, 0, 0" 0.001) (Math|Boolean|Equal(Boolean) (and (<= (Math|Vector|VectorLength (- (.location _returnvalue_10) (Transformation|GetActorLocation))) (* (Variables|Default|GetDistanceThreshold) _returnvalue_7)) (<= (Math|Vector|DotProduct (Math|Vector|GetForwardVector (.rotation _returnvalue_10)) (Math|Vector|GetForwardVector (Variables|Default|GetArrow))) (Variables|Logic|GetDotThreshold))) false))) false)))))
      (else
        (Transformation|SetActorScale3D _returnvalue_4)
        (if (Math|Vector|Equal(Vector) _returnvalue_4 "0, 0, 0" 0.001)
          (Actor|DestroyActor))))))

(fn ConstructionScript
  (CallFunction|UpdateHelperParameters))

(fn UpdateHelperParameters
  (bind _linethickness (Variables|Line|GetLineThickness))
  (bind _linethickness_2 (Variables|Line|GetLineThickness))
  (bind _text (Variables|Text|GetText))
  (bind _textscale (Variables|Text|GetTextScale))
  (bind _textscale_2 (Variables|Text|GetTextScale))
  (bind _text_2 (Variables|Text|GetText))
  (bind _baselinelength (Variables|Line|GetBaseLineLength))
  (bind _returnvalue (Utilities|String|ToString(Text) _text))
  (bind _returnvalue_2 (Math|Float|NormalizetoRange _textscale 1.0 4.0))
  (bind _returnvalue_3 (Math|Float|NormalizetoRange _textscale_2 1.0 4.0))
  (bind _returnvalue_4 (Utilities|String|ToString(Text) _text_2))
  (bind _returnvalue_5 (Math|Float|Lerp 0.4 1.448442 _returnvalue_3))
  (bind _returnvalue_6 (Math|Float|Lerp 3.2 1.34 _returnvalue_2))
  (bind _returnvalue_7 (Utilities|String|Len _returnvalue_4))
  (bind _returnvalue_8 (Utilities|String|Len _returnvalue))
  (bind _returnvalue_9 (Math|Conversions|ToFloat(Integer) _returnvalue_8))
  (bind _returnvalue_10 (Math|Float|NormalizetoRange _returnvalue_9 0.0 5e+01))
  (bind _returnvalue_11 (Math|Float|Lerp 1.5 0.9 _returnvalue_10))
  (bind _returnvalue_12 (* _returnvalue_7 _returnvalue_11))
  (bind _returnvalue_13 (/ _returnvalue_12 _returnvalue_6))
  (SplineMesh|SetStartandEnd (Variables|Default|GetBase) "0, 0, 0" (Math|Vector|MakeVector _baselinelength 0.0 0.0) (Math|Vector|MakeVector _baselinelength 0.0 0.0) (Math|Vector|MakeVector _baselinelength 0.0 0.0) true :!class /Script/Engine.SplineMeshComponent)
  (Rendering|Components|TextRender|SetText (Variables|Default|GetTextRender) (Variables|Text|GetText))
  (Rendering|Components|TextRender|SetWorldSize (Variables|Default|GetTextRender) (Variables|Text|GetTextScale))
  (SplineMesh|SetEndScale (Variables|Default|GetBase) (Math|Vector2D|MakeVector2D _linethickness_2 _linethickness_2) true :!class /Script/Engine.SplineMeshComponent)
  (SplineMesh|SetStartScale (Variables|Default|GetBase) (Math|Vector2D|MakeVector2D _linethickness _linethickness) true :!class /Script/Engine.SplineMeshComponent)
  (Transformation|SetRelativeRotation (Variables|Default|GetArrow) (Variables|Line|GetRotation) false false)
  (Transformation|SetRelativeLocation (Variables|Default|GetT_TextUnderline) (Math|Vector|MakeVector (Variables|Line|GetBaseLineLength) 0.0 0.0) false false)
  (Transformation|SetRelativeScale3D (Variables|Default|GetSM_BG_Center) (Math|Vector|MakeVector _returnvalue_12 1.0 1.0))
  (Transformation|SetRelativeLocation (Variables|Default|GetTextRender) (Math|Vector|MakeVector 0.0 (Utilities|Select :Index (Variables|Text|GetAlignment) :EHTA_Left (/ _returnvalue_12 (* _returnvalue_6 -1.0)) :EHTA_Center _returnvalue_13 :EHTA_Right _returnvalue_13) 0.0) false false)
  (Transformation|SetRelativeLocation (Variables|Default|GetSM_BG_Right) (Math|Vector|MakeVector 0.0 (- (* _returnvalue_12 -1.0) 0.501) 0.0) false false)
  (Transformation|SetRelativeScale3D (Variables|Default|GetT_BG) (Math|Vector|MakeVector _returnvalue_5 (Utilities|Select :Index (Variables|Text|GetAlignment) :EHTA_Left _returnvalue_5 :EHTA_Center _returnvalue_5 :EHTA_Right (* _returnvalue_5 -1.0)) _returnvalue_5)))