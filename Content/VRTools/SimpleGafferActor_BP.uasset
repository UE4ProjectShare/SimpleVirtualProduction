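; Gaffer spotlight actor for VR tools, with preset brightness, cone radius and color temperature options selected by index.
; Setters drive the SpotLight and mirror power and temperature on the housing's dynamic material, created in Init.
; Radius also rotates four barn door flaps to match.
; NextColorTemperature steps through presets inside an undoable transaction, while NextRadius and NextBrightness are empty stubs.
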(event EventBeginPlay)

(event Collision|EventActorBeginOverlap
  (params (OtherActor :type Actor%20Object%20Reference)))

(event EventTick
  (params (DeltaSeconds :type Float%20%28single-precision%29)))

(fn ConstructionScript)

(fn NextColorTemperature
  (params (bTemperatureUp :type Boolean))
  (if bTemperatureUp
    (LocalVariables|SetTemperatureChange 1)
    (else
      (LocalVariables|SetTemperatureChange -1)))
  (Utilities|CreateTransaction "" "Change Temperature" :!label _label
    (:Pending
      (Transactions|TransactObject self)
      (bind _output_get (Variables|Default|SetCurrentTemperatureIndex (Math|Integer|Clamp(Integer) (+ (Variables|Default|GetCurrentTemperatureIndex) (LocalVariables|GetTemperatureChange)) 0 (- (Utilities|Array|Length (Variables|Default|GetTemperatureOptions)) 1))))
      (Class|LightComponent|SetTemperature (Variables|Default|GetSpotLight) (Utilities|Array|Get(acopy) (Variables|Default|GetTemperatureOptions) _output_get))
      (bind _output_get_2 (Variables|Default|SetcurrentNormalizedTemperature (Math|Float|Clamp(Float) (Math|Float|NormalizetoRange (Utilities|Array|Get(acopy) (Variables|Default|GetTemperatureOptions) _output_get) (Variables|Default|GettempRangeMin) (Variables|Default|GettempRangeMax)))))
      (Rendering|Material|SetScalarParameterValue (Variables|Default|GetDMI_Gaffer) "Temperature" _output_get_2 :!class /Script/Engine.MaterialInstanceDynamic)
      (goto _label Finalize))
    (:Complete
      (return (Utilities|Array|Get(acopy) (Variables|Default|GetTemperatureOptions) _output_get) (Variables|Default|GetcurrentNormalizedTemperature)))))

(fn NextRadius
  (params (bRadiusUp :type Boolean))
  (return 0.0))

(fn NextBrightness
  (params (bBrightnessUp :type Boolean)))

(fn ConvertLumenstoWatts
  (params (Lumens :type Float%20%28single-precision%29))
  (return (* Lumens 15.0)))

(fn ConvertWattstoLumens
  (params (Watts :type Float%20%28single-precision%29))
  (return (/ Watts 15.0)))

(fn NormalizeRadiusOptions
  (params (Value :type Float%20%28single-precision%29))
  (return (Math|Float|Lerp 0.0 9e+01 (Math|Float|NormalizetoRange Value 15.0 1.8e+02))))

(fn Init
  (bind _sm_gaffer_light (Variables|Default|GetSM_Gaffer_Light))
  (bind _returnvalue (Rendering|Material|CreateDynamicMaterialInstance _sm_gaffer_light 0 (Rendering|Material|GetMaterial _sm_gaffer_light 0) "None" :!class /Script/Engine.PrimitiveComponent))
  (Variables|Default|SetDMI_Gaffer _returnvalue))

(fn SetBarnDoorsAngle
  (Transformation|SetRelativeRotation (Variables|Default|GetSM_Gaffer_Flap_1) (Math|Rotator|MakeRotator 0.0 (CallFunction|NormalizeRadiusOptions (Utilities|Array|Get(acopy) (Variables|Default|GetRadiusOptions) (Variables|Default|GetCurrentRadiusIndex))) 0.0) false false)
  (Transformation|SetRelativeRotation (Variables|Default|GetSM_Gaffer_Flap_2) (Math|Rotator|MakeRotator 0.0 0.0 (* (CallFunction|NormalizeRadiusOptions (Utilities|Array|Get(acopy) (Variables|Default|GetRadiusOptions) (Variables|Default|GetCurrentRadiusIndex))) -1.0)) false false)
  (Transformation|SetRelativeRotation (Variables|Default|GetSM_Gaffer_Flap_4) (Math|Rotator|MakeRotator 0.0 (* (CallFunction|NormalizeRadiusOptions (Utilities|Array|Get(acopy) (Variables|Default|GetRadiusOptions) (Variables|Default|GetCurrentRadiusIndex))) -1.0) 0.0) false false)
  (Transformation|SetRelativeRotation (Variables|Default|GetSM_Gaffer_Flap_3) (Math|Rotator|MakeRotator 0.0 0.0 (CallFunction|NormalizeRadiusOptions (Utilities|Array|Get(acopy) (Variables|Default|GetRadiusOptions) (Variables|Default|GetCurrentRadiusIndex)))) false false))

(fn SetBrightness
  (params (BrightnessIndex :type Integer))
  (bind _brightnessoptions (Variables|Default|GetBrightnessOptions))
  (bind _output (Utilities|Array|Get(acopy) _brightnessoptions BrightnessIndex))
  (Variables|Default|SetCurrentBrightnessIndex BrightnessIndex)
  (Rendering|Components|Light|SetIntensity (Variables|Default|GetSpotLight) _output)
  (Rendering|Material|SetScalarParameterValue (Variables|Default|GetDMI_Gaffer) "Power" (Math|Float|Lerp 25.0 5e+02 (Math|Float|NormalizetoRange _output 1.5e+02 2e+04)) :!class /Script/Engine.MaterialInstanceDynamic))

(fn SetRadius
  (params (RadiusIndex :type Integer))
  (Variables|Default|SetCurrentRadiusIndex RadiusIndex)
  (Rendering|Lighting|SetOuterConeAngle (Variables|Default|GetSpotLight) (/ (Utilities|Array|Get(acopy) (Variables|Default|GetRadiusOptions) RadiusIndex) 2.0))
  (CallFunction|SetBarnDoorsAngle))

(fn SetColorTemperature
  (params (TemperatureIndex :type Integer))
  (bind _temperatureoptions (Variables|Default|GetTemperatureOptions))
  (bind _output (Utilities|Array|Get(acopy) _temperatureoptions TemperatureIndex))
  (Variables|Default|SetCurrentTemperatureIndex TemperatureIndex)
  (Class|LightComponent|SetTemperature (Variables|Default|GetSpotLight) _output)
  (Rendering|Material|SetScalarParameterValue (Variables|Default|GetDMI_Gaffer) "Temperature" (Math|Float|Clamp(Float) (Math|Float|NormalizetoRange _output 1.7e+03 1.2e+04)) :!class /Script/Engine.MaterialInstanceDynamic))